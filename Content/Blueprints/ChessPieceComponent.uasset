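; Actor component for chess pieces that links generic calls to the specific piece character that owns it.
; ParentHighlightMoves switches on ComponentTitle and casts the owner to the matching piece class, but only Pawn calls HilightMoves, with glow fixed to false.
; Other cases stop after the cast, ignoring the event's inputs.
; GetParent returns the owner as typed Pawn and Knight outputs, handling only those two types.
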(event Custom|ParentHighlightMoves
  (params (OriginTile :type Smart%20Tile%20Tile%20Map%20Object%20Reference) (GlowOn :type Boolean))
  (bind _returnvalue (Components|GetOwner))
  (switch Utilities|FlowControl|Switch|Switchonpiece_titles (Variables|Default|GetComponentTitle)
    (:NewEnumerator0
      (bind _aspawn_pchar (Utilities|Casting|CastTopawn_PChar _returnvalue))
      (Default|HilightMoves _aspawn_pchar 0 false))
    (:NewEnumerator1
      (Utilities|Casting|CastToknight_PChar _returnvalue))
    (:NewEnumerator2
      (Utilities|Casting|CastTobishop_PChar _returnvalue))
    (:NewEnumerator3
      (Utilities|Casting|CastTorook_PChar _returnvalue))
    (:NewEnumerator4
      (Utilities|Casting|CastToqueen_PChar _returnvalue))
    (:NewEnumerator5
      (Utilities|Casting|CastToking_PChar _returnvalue))
    (:NewEnumerator6
      (Utilities|Casting|CastTopiece_PaperChar _returnvalue))))

(event EventBeginPlay)

(event EventTick
  (params (DeltaSeconds :type Float%20%28single-precision%29)))

(fn GetParent
  (bind _returnvalue (Components|GetOwner))
  (switch Utilities|FlowControl|Switch|Switchonpiece_titles (Variables|Default|GetComponentTitle)
    (:NewEnumerator0
      (bind _aspawn_pchar (Utilities|Casting|CastTopawn_PChar _returnvalue)
        (:then
          _)
        (:CastFailed
          _)))
    (:NewEnumerator1
      (bind _asknight_pchar (Utilities|Casting|CastToknight_PChar _returnvalue)
        (:then
          _)
        (:CastFailed
          _))))
  (return _aspawn_pchar _asknight_pchar 0))