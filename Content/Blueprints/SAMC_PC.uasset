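; SAMC_PC is the player controller for a chess game, handling turn order, check detection and popup widgets.
; ChangeTurn flips the turn token, then queries the kings: a player ending their turn in check loses, while a checked opponent gets an alert.
; VarsComponent holds turn, board and body-count state, which save loading restores before refreshing the scoreboard.
; The mouse drag and overlap debug logic in EventGraph never runs.
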(event EventBeginPlay
  (Development|PrintString "SAMC_PC loaded" true true "(R=0.003705,G=1.000000,B=0.258819,A=1.000000)")
  (Default|CallNewLevelLoaded))

(event EventTick
  (params (DeltaSeconds :type Float%20%28single-precision%29)))

(event Input|MouseEvents|LeftMouseButton
  (params (Key :type Key%20Structure :default "AnyKey")))

(event Custom|CreateLosePopup
  (params (LosingTeam :type team%20Enum))
  (bind _returnvalue (UserInterface|CreateWidget "/Game/Blueprints/EndGameAlertWidget.EndGameAlertWidget_C" self (Utilities|Text|ToText(String) (Utilities|String|Append (CallFunction|ToTitle (Utilities|String|EnumtoString (CallFunction|OppositeTeam LosingTeam))) " Wins!")) (Utilities|Text|ToText(String) (Utilities|String|Append (CallFunction|ToTitle (Utilities|String|EnumtoString LosingTeam)) " Lost!"))))
  (UserInterface|Viewport|AddtoViewport _returnvalue 10))

(event Custom|CreateNYTPopup
  (bind _returnvalue (UserInterface|CreateWidget "/Game/Blueprints/NYTPopup.NYTPopup_C" self))
  (UserInterface|Viewport|AddtoViewport _returnvalue 0))

(event Custom|CreateCheatersPopup
  (bind _returnvalue (UserInterface|CreateWidget "/Game/Blueprints/VolatilePopup.VolatilePopup_C" self))
  (UserInterface|Viewport|AddtoViewport _returnvalue 0))

(fn ConstructionScript)

(fn ChangeTurn
  (bind _varscomponent (Variables|Default|GetVarsComponent))
  (Development|PrintString (Utilities|String|Append "**************Changing turn from " (Utilities|String|EnumtoString (Variables|/Game/Blueprints/VarsComponent.VarsComponent_C|GetTurn_Token _varscomponent))) true true "(R=0.000000,G=0.660000,B=1.000000,A=1.000000)" 6.0)
  (switch Utilities|FlowControl|Switch|Switchonteam (Variables|/Game/Blueprints/VarsComponent.VarsComponent_C|GetTurn_Token _varscomponent)
    (:NewEnumerator0
      (Variables|/Game/Blueprints/VarsComponent.VarsComponent_C|SetTurn_Token _varscomponent "NewEnumerator1")
      (Utilities|CheckforCheckMacro "NewEnumerator0"
        (:True
          (Development|PrintString "THE WHITE KING IS IN CHECK" true true "(R=1.000000,G=0.000000,B=0.000000,A=1.000000)" 2e+01)
          (CallFunction|ThrowLosePopup "White lost!" "Black Wins!"))
        (:False
          (Utilities|CheckforCheckMacro "NewEnumerator1"
            (:True
              (Development|PrintString "THE BLACK KING IS IN CHECK" true true "(R=1.000000,G=0.000000,B=0.000000,A=1.000000)" 2e+01)
              (CallFunction|ThrowAlertPopup "The Black king is in check!" "I'll Handle This!"))
            (:False
              (bind _dangerclose (Default|CheckforCheck (Variables|Default|GetWhite_King) :!label _label))
              (bind _output_get (Variables|Default|Setwhite_in_check _dangerclose))
              (if _output_get
                (Development|PrintString "THE WHITE KING IS IN CHECK" true true "(R=1.000000,G=0.000000,B=0.000000,A=1.000000)" 2e+01)
                (CallFunction|ThrowAlertPopup "The White king is in check!" "I'll Handle This!")))))))
    (:NewEnumerator1
      (Variables|/Game/Blueprints/VarsComponent.VarsComponent_C|SetTurn_Token _varscomponent "NewEnumerator0")
      (bind _dangerclose_2 (Default|CheckforCheck (Variables|Default|GetBlack_King)))
      (bind _output_get_2 (Variables|Default|Setblack_in_check _dangerclose_2))
      (if _output_get_2
        (Development|PrintString "THE BLACK KING IS IN CHECK" true true "(R=1.000000,G=0.000000,B=0.000000,A=1.000000)" 2e+01)
        (CallFunction|ThrowLosePopup "Black lost!" "White Wins!")
        (else
          (goto _label))))))

(fn GetTurn
  (return (Variables|/Game/Blueprints/VarsComponent.VarsComponent_C|GetTurn_Token (Variables|Default|GetVarsComponent))))

(fn SetKing
  (params (king_piece :type King%20P%20Char%20Object%20Reference))
  (switch Utilities|FlowControl|Switch|Switchonteam (Variables|/Game/PaperChars/piece_PaperChar.piece_PaperChar_C|Getteam king_piece)
    (:NewEnumerator0
      (Variables|Default|SetWhite_King king_piece))
    (:NewEnumerator1
      (Variables|Default|SetBlack_King king_piece))))

(fn GetKinginCheck
  (return (Utilities|Select :Index (CallFunction|GetTurn) :NewEnumerator0 (Variables|Default|Getwhite_in_check) :NewEnumerator1 (Variables|Default|Getblack_in_check) :NewEnumerator2 false)))

(fn ThrowAlertPopup
  (params (AlertText :type Text) (AlertButtonText :type Text))
  (bind _returnvalue (UserInterface|CreateWidget "/Game/Blueprints/AlertWidget.AlertWidget_C" self AlertText AlertButtonText))
  (UserInterface|Viewport|AddtoViewport _returnvalue 0)
  (return))

(fn ThrowLosePopup
  (params (AlertText :type Text) (AlertButtonText :type Text))
  (bind _returnvalue (UserInterface|CreateWidget "/Game/Blueprints/EndGameAlertWidget.EndGameAlertWidget_C" self AlertText AlertButtonText))
  (UserInterface|Viewport|AddtoViewport _returnvalue 0)
  (return))

(fn RegisterBoard
  (params (BoardToRegister :type Board%20Tile%20Map%20Object%20Reference))
  (bind _varscomponent (Variables|Default|GetVarsComponent))
  (Variables|/Game/Blueprints/VarsComponent.VarsComponent_C|SetRootBoard _varscomponent BoardToRegister)
  (Variables|/Game/Blueprints/VarsComponent.VarsComponent_C|Setboard_is_set _varscomponent true)
  (Default|CallBoardGotRegisted)
  (return))

(fn GetBoard
  (return (Variables|/Game/Blueprints/VarsComponent.VarsComponent_C|GetRootBoard (Variables|Default|GetVarsComponent))))

(fn LoadfromSave
  (params (SlotName :type String) (UserIndex :type Integer))
  (bind _returnvalue (SaveGame|LoadGamefromSlot SlotName UserIndex))
  (bind _assamc_save_game (Utilities|Casting|CastToSAMC_SaveGame _returnvalue))
  (CallFunction|LoadfromSaveObject _assamc_save_game)
  (return))

(fn CheatersPopup
  (bind _returnvalue (UserInterface|CreateWidget "/Game/Blueprints/VolatilePopup.VolatilePopup_C" self))
  (UserInterface|Viewport|AddtoViewport _returnvalue 0))

(fn NotYourTurnPopup
  (bind _returnvalue (UserInterface|CreateWidget "/Game/Blueprints/NYTPopup.NYTPopup_C" self))
  (UserInterface|Viewport|AddtoViewport _returnvalue 0))

(fn LoadfromSaveObject
  (params (NewSaveGame :type SAMC%20Save%20Game%20Object%20Reference))
  (LocalVariables|SetLoadedSavegame NewSaveGame)
  (Variables|/Game/Blueprints/VarsComponent.VarsComponent_C|SetTurn_Token (Variables|Default|GetVarsComponent) (Variables|/Game/Blueprints/SAMC_SaveGame.SAMC_SaveGame_C|GetCurrentTurn (LocalVariables|GetLoadedSavegame)))
  (bind _registeredboard (CallFunction|GetBoard))
  (Default|UnpackBoard _registeredboard (Variables|/Game/Blueprints/SAMC_SaveGame.SAMC_SaveGame_C|GetSavedTiles (LocalVariables|GetLoadedSavegame)))
  (bind _output_get (Variables|/Game/Blueprints/VarsComponent.VarsComponent_C|SetBodyCountCollection (Variables|Default|GetVarsComponent) (Variables|/Game/Blueprints/SAMC_SaveGame.SAMC_SaveGame_C|GetSavedBodyCount (LocalVariables|GetLoadedSavegame))))
  (Default|CallNewLevelLoaded)
  (Default|UpdateScores (Variables|Default|GetMyScoreBoard) _output_get)
  (return))