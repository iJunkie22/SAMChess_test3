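; Chess game HUD that draws the SAMchess title and White/Black labels, highlighting the side to move in white, or red when a king is in check.
; DrawHUD anchors the layout to a fixed world point projected to screen, scales it by viewport, and centers labels via measured text size.
; BeginPlay caches SAMC_PC and binds its new-level event to spawn the ScoreBoard widget.
; CalcHudRowPosition is a stub.
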(event Custom|SpawnScoreBoard
  (bind _returnvalue (UserInterface|CreateWidget "/Game/Blueprints/ScoreBoard.ScoreBoard_C" (stale EventBeginPlay _output_get)))
  (UserInterface|Viewport|AddtoViewport _returnvalue 0)
  (Variables|/Game/Blueprints/SAMC_PC.SAMC_PC_C|SetMyScoreBoard (Variables|Default|GetMyPC) _returnvalue))

(event EventBeginPlay
  (bind _assamc_pc (Utilities|Casting|CastToSAMC_PC (Game|GetPlayerController 0))
    (:then
      (bind _output_get (Variables|Default|SetMyPC _assamc_pc))
      (CallFunction|CalcHudOffset)
      (EventDispatchers|BindEventtoNewLevelLoaded _output_get (delegate Custom|SpawnScoreBoard))
      (Default|CallNewLevelLoaded (Variables|Default|GetMyPC)))
    (:CastFailed
      (Development|PrintString "****SAMC_PC init failed for HUD" true true "(R=1.000000,G=0.033320,B=0.000000,A=1.000000)" 12.0))))

(event EventActorBeginOverlap
  (params (OtherActor :type Actor%20Object%20Reference)))

(event EventTick
  (params (DeltaSeconds :type Float%20%28single-precision%29)))

(event EventDrawHUD
  (params (SizeX :type Integer) (SizeY :type Integer))
  (bind _scaledsize (CallFunction|GetTitleSize))
  (bind _returnscale (CallFunction|GetIdealViewportScale))
  (bind _offsetresult (CallFunction|CalcHudOffset))
  (Class|HUD|DrawTextureSimple "/Game/UI_Stuff/MenuStuff/SAMchess_title.SAMchess_title" (.X (Math|Vector2D|BreakVector2D _offsetresult)) (.Y (Math|Vector2D|BreakVector2D _offsetresult)) _returnscale false)
  (HUD|DrawRect (select (Default|GetKinginCheck (Variables|Default|GetMyPC)) "(R=1.000000,G=0.000000,B=0.084117,A=1.000000)" "(R=1.000000,G=1.000000,B=1.000000,A=1.000000)") (.Origin_X (Utilities|Struct|Break2DPositionedBox (Utilities|Select :Index (Default|GetTurn (Variables|Default|GetMyPC)) :NewEnumerator0 (.2DPosBox (CallFunction|StringAlignCenter "White" (.X (Math|Vector2D|BreakVector2D (+ _offsetresult _scaledsize))) (.Y (Math|Vector2D|BreakVector2D (+ _offsetresult _scaledsize))) "/Game/UI_Stuff/Fonts/Quango.Quango" _returnscale)) :NewEnumerator1 (.2DPosBox (CallFunction|StringAlignCenter "Black" (.X (Math|Vector2D|BreakVector2D _offsetresult)) (+ (.Y (Math|Vector2D|BreakVector2D _offsetresult)) (.Y (Math|Vector2D|BreakVector2D _scaledsize))) "/Game/UI_Stuff/Fonts/Quango.Quango" _returnscale)) :NewEnumerator2 ""))) (.Origin_Y (Utilities|Struct|Break2DPositionedBox (Utilities|Select :Index (Default|GetTurn (Variables|Default|GetMyPC)) :NewEnumerator0 (.2DPosBox (CallFunction|StringAlignCenter "White" (.X (Math|Vector2D|BreakVector2D (+ _offsetresult _scaledsize))) (.Y (Math|Vector2D|BreakVector2D (+ _offsetresult _scaledsize))) "/Game/UI_Stuff/Fonts/Quango.Quango" _returnscale)) :NewEnumerator1 (.2DPosBox (CallFunction|StringAlignCenter "Black" (.X (Math|Vector2D|BreakVector2D _offsetresult)) (+ (.Y (Math|Vector2D|BreakVector2D _offsetresult)) (.Y (Math|Vector2D|BreakVector2D _scaledsize))) "/Game/UI_Stuff/Fonts/Quango.Quango" _returnscale)) :NewEnumerator2 ""))) (.Width (Utilities|Struct|Break2DPositionedBox (Utilities|Select :Index (Default|GetTurn (Variables|Default|GetMyPC)) :NewEnumerator0 (.2DPosBox (CallFunction|StringAlignCenter "White" (.X (Math|Vector2D|BreakVector2D (+ _offsetresult _scaledsize))) (.Y (Math|Vector2D|BreakVector2D (+ _offsetresult _scaledsize))) "/Game/UI_Stuff/Fonts/Quango.Quango" _returnscale)) :NewEnumerator1 (.2DPosBox (CallFunction|StringAlignCenter "Black" (.X (Math|Vector2D|BreakVector2D _offsetresult)) (+ (.Y (Math|Vector2D|BreakVector2D _offsetresult)) (.Y (Math|Vector2D|BreakVector2D _scaledsize))) "/Game/UI_Stuff/Fonts/Quango.Quango" _returnscale)) :NewEnumerator2 ""))) (.Height (Utilities|Struct|Break2DPositionedBox (Utilities|Select :Index (Default|GetTurn (Variables|Default|GetMyPC)) :NewEnumerator0 (.2DPosBox (CallFunction|StringAlignCenter "White" (.X (Math|Vector2D|BreakVector2D (+ _offsetresult _scaledsize))) (.Y (Math|Vector2D|BreakVector2D (+ _offsetresult _scaledsize))) "/Game/UI_Stuff/Fonts/Quango.Quango" _returnscale)) :NewEnumerator1 (.2DPosBox (CallFunction|StringAlignCenter "Black" (.X (Math|Vector2D|BreakVector2D _offsetresult)) (+ (.Y (Math|Vector2D|BreakVector2D _offsetresult)) (.Y (Math|Vector2D|BreakVector2D _scaledsize))) "/Game/UI_Stuff/Fonts/Quango.Quango" _returnscale)) :NewEnumerator2 ""))))
  (HUD|DrawText (.TextOut (CallFunction|StringAlignCenter "White" (.X (Math|Vector2D|BreakVector2D (+ _offsetresult _scaledsize))) (.Y (Math|Vector2D|BreakVector2D (+ _offsetresult _scaledsize))) "/Game/UI_Stuff/Fonts/Quango.Quango" _returnscale)) "(R=0,G=0,B=0,A=1)" (.OriginX (CallFunction|StringAlignCenter "White" (.X (Math|Vector2D|BreakVector2D (+ _offsetresult _scaledsize))) (.Y (Math|Vector2D|BreakVector2D (+ _offsetresult _scaledsize))) "/Game/UI_Stuff/Fonts/Quango.Quango" _returnscale)) (.OriginY (CallFunction|StringAlignCenter "White" (.X (Math|Vector2D|BreakVector2D (+ _offsetresult _scaledsize))) (.Y (Math|Vector2D|BreakVector2D (+ _offsetresult _scaledsize))) "/Game/UI_Stuff/Fonts/Quango.Quango" _returnscale)) (.FontOut (CallFunction|StringAlignCenter "White" (.X (Math|Vector2D|BreakVector2D (+ _offsetresult _scaledsize))) (.Y (Math|Vector2D|BreakVector2D (+ _offsetresult _scaledsize))) "/Game/UI_Stuff/Fonts/Quango.Quango" _returnscale)) (.ScaleOut (CallFunction|StringAlignCenter "White" (.X (Math|Vector2D|BreakVector2D (+ _offsetresult _scaledsize))) (.Y (Math|Vector2D|BreakVector2D (+ _offsetresult _scaledsize))) "/Game/UI_Stuff/Fonts/Quango.Quango" _returnscale)) false)
  (HUD|DrawText (.TextOut (CallFunction|StringAlignCenter "Black" (.X (Math|Vector2D|BreakVector2D _offsetresult)) (+ (.Y (Math|Vector2D|BreakVector2D _offsetresult)) (.Y (Math|Vector2D|BreakVector2D _scaledsize))) "/Game/UI_Stuff/Fonts/Quango.Quango" _returnscale)) "(R=0,G=0,B=0,A=1)" (.OriginX (CallFunction|StringAlignCenter "Black" (.X (Math|Vector2D|BreakVector2D _offsetresult)) (+ (.Y (Math|Vector2D|BreakVector2D _offsetresult)) (.Y (Math|Vector2D|BreakVector2D _scaledsize))) "/Game/UI_Stuff/Fonts/Quango.Quango" _returnscale)) (.OriginY (CallFunction|StringAlignCenter "Black" (.X (Math|Vector2D|BreakVector2D _offsetresult)) (+ (.Y (Math|Vector2D|BreakVector2D _offsetresult)) (.Y (Math|Vector2D|BreakVector2D _scaledsize))) "/Game/UI_Stuff/Fonts/Quango.Quango" _returnscale)) (.FontOut (CallFunction|StringAlignCenter "Black" (.X (Math|Vector2D|BreakVector2D _offsetresult)) (+ (.Y (Math|Vector2D|BreakVector2D _offsetresult)) (.Y (Math|Vector2D|BreakVector2D _scaledsize))) "/Game/UI_Stuff/Fonts/Quango.Quango" _returnscale)) (.ScaleOut (CallFunction|StringAlignCenter "Black" (.X (Math|Vector2D|BreakVector2D _offsetresult)) (+ (.Y (Math|Vector2D|BreakVector2D _offsetresult)) (.Y (Math|Vector2D|BreakVector2D _scaledsize))) "/Game/UI_Stuff/Fonts/Quango.Quango" _returnscale)) false))

(fn ConstructionScript)

(fn CalcHudOffset
  (params (PlayerControllerNumber :type Integer))
  (bind _returnvalue (Game|GetPlayerController PlayerControllerNumber))
  (bind (_screenlocation _returnvalue_2) (Class|PlayerController|ProjectWorldLocationtoScreen _returnvalue "2070.000000,0.000000,-70.000000"))
  (bind (_x _y) (Math|Vector2D|BreakVector2D _screenlocation))
  (return (Math|Vector2D|MakeVector2D _x (* _y (Class|WidgetLayoutLibrary|GetViewportScale))) _returnvalue_2))

(fn CalcHudRowPosition
  (params (OriginOffset :type Vector%202D%20Structure) (RowHeight :type Float%20%28single-precision%29) (RowIndex :type Integer) (RowPadding :type Float%20%28single-precision%29))
  (return 0.0 0.0))

(fn StringAlignCenter
  (params (TextToDisplay :type String) (CenterX :type Float%20%28single-precision%29) (CenterY :type Float%20%28single-precision%29) (Font :type Font%20Object%20Reference) (Scale :type Float%20%28single-precision%29))
  (bind (_outwidth _outheight) (Class|HUD|GetTextSize TextToDisplay Font Scale))
  (bind _returnvalue (/ _outwidth 2.0))
  (bind _returnvalue_2 (/ _outheight 2.0))
  (bind _returnvalue_3 (- CenterX _returnvalue))
  (bind _returnvalue_4 (- CenterY _returnvalue_2))
  (return _returnvalue_3 _returnvalue_4 _outwidth _outheight Font Scale TextToDisplay (Utilities|Struct|Make2DPositionedBox _returnvalue_3 _returnvalue_4 _outwidth _outheight)))

(fn DrawCenteredText
  (params (TextToDisplay :type String) (CenterX :type Float%20%28single-precision%29) (CenterY :type Float%20%28single-precision%29) (Font :type Font%20Object%20Reference) (Scale :type Float%20%28single-precision%29) (Color :type Linear%20Color%20Structure))
  (bind (_originx _originy _width _height _fontout _scaleout _textout _2dposbox) (CallFunction|StringAlignCenter TextToDisplay CenterX CenterY Font Scale))
  (HUD|DrawText _textout Color _originx _originy _fontout _scaleout false)
  (return _2dposbox))

(fn GetTitleSize
  (return (* (Variables|Default|GetSAMC_Title_size) (CallFunction|GetIdealViewportScale))))

(fn GetIdealViewportScale
  (return (/ (Class|WidgetLayoutLibrary|GetViewportScale) 0.66666)))