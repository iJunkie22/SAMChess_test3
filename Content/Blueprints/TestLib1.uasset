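; Function library for a Paper2D chess game, handling captured-piece tallies, spawning and board-state packing.
; Body count getters and setters index by title and team, with the setter converting the struct to an array and back.
; PieceFactory spawns a piece by title, initializes it and assigns it to its tile; TileFactory picks dark or light tiles by coordinate-product parity.
; PiecePack converts a tile's occupant into a tile data struct.
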(fn GetBodyCount
  (params (BodyCountStruct :type SAMC%20Body%20Count%20Data%20Struct%20Structure%20%28by%20ref%29) (TargetTeam :type team%20Enum) (TargetTitle :type piece_titles%20Enum))
  (bind (_deadblackpawns _deadwhitepawns _deadblackbishops _deadwhitebishops _deadblackrooks _deadwhiterooks _deadblackknights _deadwhiteknights _deadblackqueens _deadwhitequeens _deadblackkings _deadwhitekings) (Utilities|Struct|BreakSAMC_BodyCount_DataStruct BodyCountStruct))
  (if (Validation|ValidTeam TargetTeam)
    (if (Validation|ValidPieceTitle TargetTitle)
      (return (Utilities|Select :Index (+ (* (Utilities|Select :Index TargetTitle :NewEnumerator0 0 :NewEnumerator1 3 :NewEnumerator2 1 :NewEnumerator3 2 :NewEnumerator4 4 :NewEnumerator5 5 :NewEnumerator6 -99) 2) (Utilities|Select :Index TargetTeam :NewEnumerator0 1 :NewEnumerator1 0 :NewEnumerator2 -99)) :Option%200 _deadblackpawns :Option%201 _deadwhitepawns :Option%202 _deadblackbishops :Option%203 _deadwhitebishops :Option%204 _deadblackrooks :Option%205 _deadwhiterooks :Option%206 _deadblackknights :Option%207 _deadwhiteknights :Option%208 _deadblackqueens :Option%209 _deadwhitequeens :Option%2010 _deadblackkings :Option%2011 _deadwhitekings) TargetTeam TargetTitle)
      (else
        _)))
  (return -99999 TargetTeam TargetTitle))

(fn ValidTeam
  (params (TestTeam :type team%20Enum%20%28by%20ref%29))
  (return (Utilities|Enum|NotEqual(Enum) TestTeam (Utilities|Enum|Literalenumteam "NewEnumerator2"))))

(fn ValidPieceTitle
  (params (TestTitle :type piece_titles%20Enum))
  (return (Utilities|Enum|NotEqual(Enum) TestTitle (Utilities|Enum|Literalenumpiece_titles "NewEnumerator6"))))

(fn SetBodyCount
  (params (BodyCountStruct :type SAMC%20Body%20Count%20Data%20Struct%20Structure%20%28by%20ref%29) (TargetTeam :type team%20Enum) (TargetTitle :type piece_titles%20Enum) (CountDelta :type Integer))
  (bind _returnvalue (Utilities|Select :Index TargetTitle :NewEnumerator0 0 :NewEnumerator1 3 :NewEnumerator2 1 :NewEnumerator3 2 :NewEnumerator4 4 :NewEnumerator5 5 :NewEnumerator6 -99))
  (bind _returnvalue_2 (Utilities|Select :Index TargetTeam :NewEnumerator0 1 :NewEnumerator1 0 :NewEnumerator2 -99))
  (bind _returnvalue_3 (* _returnvalue 2))
  (bind _returnvalue_4 (+ _returnvalue_3 _returnvalue_2))
  (if (Validation|ValidTeam TargetTeam)
    (if (Validation|ValidPieceTitle TargetTitle)
      (bind _output_get (LocalVariables|SetTempBCArray (BodyCount|BodyCounttoArray BodyCountStruct)))
      (Utilities|Array|SetArrayElem _output_get _returnvalue_4 (+ (Utilities|Array|Get(acopy) _output_get _returnvalue_4) CountDelta))
      (|SetBy-RefVar BodyCountStruct (BodyCount|BodyCountfromArray (LocalVariables|GetTempBCArray)))
      (return TargetTeam TargetTitle)
      (else
        _)))
  (return TargetTeam TargetTitle))

(fn BodyCountfromArray
  (params (InputArray1 :type Array%20of%20Integers))
  (return (Utilities|Struct|MakeSAMC_BodyCount_DataStruct (Utilities|Array|Get(acopy) InputArray1) (Utilities|Array|Get(acopy) InputArray1 1) (Utilities|Array|Get(acopy) InputArray1 2) (Utilities|Array|Get(acopy) InputArray1 3) (Utilities|Array|Get(acopy) InputArray1 4) (Utilities|Array|Get(acopy) InputArray1 5) (Utilities|Array|Get(acopy) InputArray1 6) (Utilities|Array|Get(acopy) InputArray1 7) (Utilities|Array|Get(acopy) InputArray1 8) (Utilities|Array|Get(acopy) InputArray1 9) (Utilities|Array|Get(acopy) InputArray1 10) (Utilities|Array|Get(acopy) InputArray1 11))))

(fn BodyCounttoArray
  (params (InputBodyCount :type SAMC%20Body%20Count%20Data%20Struct%20Structure%20%28by%20ref%29))
  (bind (_deadblackpawns _deadwhitepawns _deadblackbishops _deadwhitebishops _deadblackrooks _deadwhiterooks _deadblackknights _deadwhiteknights _deadblackqueens _deadwhitequeens _deadblackkings _deadwhitekings) (Utilities|Struct|BreakSAMC_BodyCount_DataStruct InputBodyCount))
  (return (Utilities|Array|MakeArray _deadblackpawns _deadwhitepawns _deadblackbishops _deadwhitebishops _deadblackrooks _deadwhiterooks _deadblackknights _deadwhiteknights _deadblackqueens _deadwhitequeens _deadblackkings _deadwhitekings)))

(fn PieceFactory
  (params (StockTitle :type piece_titles%20Enum) (StockTeam :type team%20Enum) (StockIsInitPosition :type Boolean) (HomeTile :type Smart%20Tile%20Tile%20Map%20Object%20Reference%20%28by%20ref%29))
  (bind _returnvalue (Game|SpawnActorfromClass (Utilities|Select :Index StockTitle :NewEnumerator0 "/Game/PaperChars/pawn_PChar.pawn_PChar_C" :NewEnumerator1 "/Game/PaperChars/knight_PChar.knight_PChar_C" :NewEnumerator2 "/Game/PaperChars/bishop_PChar.bishop_PChar_C" :NewEnumerator3 "/Game/PaperChars/rook_PChar.rook_PChar_C" :NewEnumerator4 "/Game/PaperChars/queen_PChar.queen_PChar_C" :NewEnumerator5 "/Game/PaperChars/king_PChar.king_PChar_C" :NewEnumerator6 "/Game/PaperChars/piece_PaperChar.piece_PaperChar_C") (Math|Transform|MakeTransform (+ (Class|PaperTileMapComponent|GetTileCenterPosition (Variables|/Script/Paper2D.PaperTileMapActor|GetRenderComponent HomeTile) 0 0 0 true) "0,40.000000, 0") "0, 0, 0" "1,1,1") "AlwaysSpawn" 0 0))
  (bind _aspiece_paper_char (Utilities|Casting|CastTopiece_PaperChar _returnvalue)
    (:then
      (Variables|/Game/PaperChars/piece_PaperChar.piece_PaperChar_C|Setteam _aspiece_paper_char StockTeam)
      (Variables|/Game/PaperChars/piece_PaperChar.piece_PaperChar_C|Setis_init_location _aspiece_paper_char StockIsInitPosition)
      (Default|UpdateSkin _aspiece_paper_char)
      (Default|SetPayload HomeTile HomeTile _aspiece_paper_char)
      (switch Utilities|FlowControl|Switch|Switchonpiece_titles StockTitle
        (:NewEnumerator0
          (bind _aspawn_pchar (Utilities|Casting|CastTopawn_PChar _aspiece_paper_char)
            (:then
              (return _aspawn_pchar))
            (:CastFailed
              _)))
        (:NewEnumerator1
          (bind _asknight_pchar (Utilities|Casting|CastToknight_PChar _aspiece_paper_char)
            (:then
              (return _asknight_pchar))
            (:CastFailed
              _)))
        (:NewEnumerator2
          (bind _asbishop_pchar (Utilities|Casting|CastTobishop_PChar _aspiece_paper_char)
            (:then
              (return _asbishop_pchar))
            (:CastFailed
              _)))
        (:NewEnumerator3
          (bind _asrook_pchar (Utilities|Casting|CastTorook_PChar _aspiece_paper_char)
            (:then
              (return _asrook_pchar))
            (:CastFailed
              _)))
        (:NewEnumerator4
          (bind _asqueen_pchar (Utilities|Casting|CastToqueen_PChar _aspiece_paper_char)
            (:then
              (return _asqueen_pchar))
            (:CastFailed
              _)))
        (:NewEnumerator5
          (bind _asking_pchar (Utilities|Casting|CastToking_PChar _aspiece_paper_char)
            (:then
              (return _asking_pchar))
            (:CastFailed
              _)))
        (:NewEnumerator6
          (return _aspiece_paper_char))))
    (:CastFailed
      _))
  (Development|PrintString 0 "***CAST FAILED: PieceFactory***" true true "(R=1.000000,G=0.000000,B=0.046901,A=1.000000)" 2e+01)
  (return 0))

(fn TileFactory
  (params (RootBoard :type Board%20Tile%20Map%20Object%20Reference) (TileX :type Integer) (TileY :type Integer))
  (bind _returnvalue (Game|SpawnActorfromClass (Utilities|Select :Index (Math|Integer|%(Integer) (* (+ TileX 1) (+ TileY 1)) 2) :Option%200 "/Game/Blueprints/Actors/Board/BoardDarkTile.BoardDarkTile_C" :Option%201 "/Game/Blueprints/Actors/Board/BoardLightTile.BoardLightTile_C") (Math|Transform|MakeTransform (+ (Class|PaperTileMapComponent|GetTileCenterPosition (Variables|/Script/Paper2D.PaperTileMapActor|GetRenderComponent RootBoard) TileX TileY 0 true) "0,30.000000, 0") "0, 0, 0" "1,1,1") "AlwaysSpawn" 0 0))
  (bind _assmart_tile_tile_map (Utilities|Casting|CastToSmartTileTileMap _returnvalue)
    (:then
      (return _assmart_tile_tile_map))
    (:CastFailed
      (Development|PrintString 0 "***CAST FAILED: TileFactory***" true true "(R=1.000000,G=0.000000,B=0.046901,A=1.000000)" 2e+01)
      (return 0))))

(fn PiecePack
  (params (RootBoard :type Board%20Tile%20Map%20Object%20Reference) (TileX :type Integer) (TileY :type Integer))
  (bind (_foundtile _success) (Default|GetSmartTile RootBoard TileX TileY))
  (if _success
    (bind (_squatter _found) (Default|WhatsonMe _foundtile false false))
    (if _found
      (LocalVariables|Setresult_team (Variables|/Game/PaperChars/piece_PaperChar.piece_PaperChar_C|Getteam _squatter))
      (LocalVariables|Setresult_title (Variables|/Game/PaperChars/piece_PaperChar.piece_PaperChar_C|Getmy_title _squatter)))
    (return (Utilities|Struct|MakeSAMC_Tile_DataStruct TileX TileY (LocalVariables|Getresult_title) (LocalVariables|Getresult_team) (LocalVariables|GetResultInitLoc)))
    (else
      (Development|PrintString 0 (Utilities|String|Append "***PiecePack failed for tile (" (Utilities|String|ToString(Integer) TileX) ", " (Utilities|String|ToString(Integer) TileY) ")") true true "(R=1.000000,G=0.067961,B=0.000000,A=1.000000)" 12.0)
      (return ""))))