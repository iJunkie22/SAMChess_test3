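; SAMC_Camera is a camera actor with a view box helper based on orthographic settings.
; Its construction script pins the CameraComponent to a hard-coded world position and rotation.
; GetViewBox derives OrthoHeight from ortho width and aspect ratio, while a leftover, unused node chain projects an X-Z view corner to widget coordinates.
; BeginPlay only clears the placeholder boolean NewVar0, and Tick and overlap events are disabled.
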(event EventBeginPlay
  (Variables|Default|SetNewVar_0 false))

(event EventActorBeginOverlap
  (params (OtherActor :type Actor%20Object%20Reference)))

(event EventTick
  (params (DeltaSeconds :type Float%20%28single-precision%29)))

(fn ConstructionScript
  (Transformation|SetWorldLocationAndRotation (Variables|CameraActor|GetCameraComponent) "1720.000000,1460.000000,-680.000000" "0,-90.000000, 0" false false))

(fn GetViewBox
  (bind _cameracomponent (Variables|CameraActor|GetCameraComponent))
  (bind _output_get (LocalVariables|SetOrthoHeight (/ (Variables|/Script/Engine.CameraComponent|GetOrthoWidth _cameracomponent) (Variables|/Script/Engine.CameraComponent|GetAspectRatio _cameracomponent)))))