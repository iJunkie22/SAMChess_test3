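; BoardTileMap is a tile-map actor for an 8x8 chess-style board that registers with SAMC_PC on BeginPlay.
; InitDefaultBoard uses the ForAllTiles macro to spawn tiles and starting pieces through the tile and piece factories.
; PackUpBoard captures all 64 squares into an array, which UnpackBoard uses to respawn tiles and pieces.
; GetSmartTile finds tile actors through box overlaps at cell centres, letting piece placement work from coordinates.
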(event OnClicked(RenderComponent)
  (params (TouchedComponent :type Primitive%20Component%20Object%20Reference))
  (Development|PrintString (Utilities|String|Append "Clicked Board tile  " (Utilities|GetDisplayName TouchedComponent))))

(event EventBeginPlay
  (Development|PrintText "Spawned BoardTileMap")
  (bind _assamc_pc (Utilities|Casting|CastToSAMC_PC (Game|GetPlayerController 0)))
  (bind _output_get (Variables|Default|SetMyPC _assamc_pc))
  (Development|PrintString "registering board")
  (Default|RegisterBoard _output_get self))

(event EventActorBeginOverlap
  (params (OtherActor :type Actor%20Object%20Reference)))

(event EventTick
  (params (DeltaSeconds :type Float%20%28single-precision%29)))

(fn ConstructionScript)

(fn UsePieceFactory1
  (params (TileX :type Integer) (TileY :type Integer) (PieceTitle :type piece_titles%20Enum) (PieceTeam :type team%20Enum) (PieceIsInitLoc :type Boolean))
  (bind (_foundtile _success) (CallFunction|GetSmartTile TileX TileY))
  (if _success
    (CallFunction|PieceFactory PieceTitle PieceTeam PieceIsInitLoc _foundtile)
    (return true)
    (else
      (return false))))

(fn UsePieceFactory2
  (params (InputTileStruct :type SAMC%20Tile%20Data%20Struct%20Structure))
  (bind (_x_coord _y_coord _title _team _is_init_position) (Utilities|Struct|BreakSAMC_Tile_DataStruct InputTileStruct))
  (bind _success (Factories|UsePieceFactory1 _x_coord _y_coord _title _team _is_init_position))
  (return _success))

(fn GetSmartTile
  (params (TileX :type Integer) (TileY :type Integer))
  (bind _array (Utilities|Array|MakeArray "ObjectTypeQuery1" "ObjectTypeQuery2" "ObjectTypeQuery3"))
  (bind _rendercomponent (Variables|Default|GetRenderComponent))
  (bind _returnvalue (Class|PaperTileMapComponent|GetTileCenterPosition _rendercomponent TileX TileY 0 true))
  (bind _returnvalue_2 (+ _returnvalue "0,30.000000, 0"))
  (bind _outactors (Class|KismetSystemLibrary|BoxOverlapActorsNEW _returnvalue_2 "10.000000,100.000000,10.000000" _array "/Game/Blueprints/Actors/Board/BoardDarkTile.BoardDarkTile_C"))
  (bind _output_get (LocalVariables|Settemparray _outactors))
  (bind _outactors_2 (Class|KismetSystemLibrary|BoxOverlapActorsNEW _returnvalue_2 "10.000000,10.000000,10.000000" _array "/Game/Blueprints/Actors/Board/BoardLightTile.BoardLightTile_C"))
  (Utilities|Array|AppendArray _output_get _outactors_2)
  (if true
    (bind _assmart_tile_tile_map (Utilities|Casting|CastToSmartTileTileMap (Utilities|Array|Get(acopy) (LocalVariables|Gettemparray)))
      (:then
        (return _assmart_tile_tile_map true))
      (:CastFailed
        (Development|PrintString "CAST FAILED (TILE LOOKUP)" true true "(R=1.000000,G=0.093249,B=0.000000,A=1.000000)" 12.0)))
    (else
      (Development|PrintString (Utilities|String|Append "GetSmartTile Failed but found " (Utilities|String|ToString(Integer) (Utilities|Array|Length (LocalVariables|Gettemparray))) " tiles at " (Utilities|String|ToString(Vector) _returnvalue_2)) true true "(R=0.000000,G=0.660000,B=1.000000,A=1.000000)" 12.0)))
  (return 0 false))

(fn UseTileFactory1
  (params (TileX :type Integer) (TileY :type Integer))
  (bind _newtile (CallFunction|TileFactory self TileX TileY))
  (return _newtile))

(fn InitDefaultBoard
  (bind (_boardrefout _tilex _tiley) (Utilities|ForAllTiles self)
    (:LoopBody
      (bind _newsmarttile (Factories|UseTileFactory1 _boardrefout _tilex _tiley))
      (if (CallFunction|ValidPieceTitle (Utilities|Select :Index _tiley :Option%200 (Utilities|Select :Index _tilex :Option%200 "NewEnumerator3" :Option%201 "NewEnumerator1" :Option%202 "NewEnumerator2" :Option%203 "NewEnumerator5" :Option%204 "NewEnumerator4" :Option%205 "NewEnumerator2" :Option%206 "NewEnumerator1" :Option%207 "NewEnumerator3") :Option%201 "NewEnumerator0" :Option%202 "NewEnumerator6" :Option%203 "NewEnumerator6" :Option%204 "NewEnumerator6" :Option%205 "NewEnumerator6" :Option%206 "NewEnumerator0" :Option%207 (Utilities|Select :Index _tilex :Option%200 "NewEnumerator3" :Option%201 "NewEnumerator1" :Option%202 "NewEnumerator2" :Option%203 "NewEnumerator5" :Option%204 "NewEnumerator4" :Option%205 "NewEnumerator2" :Option%206 "NewEnumerator1" :Option%207 "NewEnumerator3")))
        (if (CallFunction|ValidTeam (Utilities|Select :Index _tiley :Option%200 "NewEnumerator1" :Option%201 "NewEnumerator1" :Option%202 "NewEnumerator2" :Option%203 "NewEnumerator2" :Option%204 "NewEnumerator2" :Option%205 "NewEnumerator2" :Option%206 "NewEnumerator0" :Option%207 "NewEnumerator0"))
          (CallFunction|PieceFactory (Utilities|Select :Index _tiley :Option%200 (Utilities|Select :Index _tilex :Option%200 "NewEnumerator3" :Option%201 "NewEnumerator1" :Option%202 "NewEnumerator2" :Option%203 "NewEnumerator5" :Option%204 "NewEnumerator4" :Option%205 "NewEnumerator2" :Option%206 "NewEnumerator1" :Option%207 "NewEnumerator3") :Option%201 "NewEnumerator0" :Option%202 "NewEnumerator6" :Option%203 "NewEnumerator6" :Option%204 "NewEnumerator6" :Option%205 "NewEnumerator6" :Option%206 "NewEnumerator0" :Option%207 (Utilities|Select :Index _tilex :Option%200 "NewEnumerator3" :Option%201 "NewEnumerator1" :Option%202 "NewEnumerator2" :Option%203 "NewEnumerator5" :Option%204 "NewEnumerator4" :Option%205 "NewEnumerator2" :Option%206 "NewEnumerator1" :Option%207 "NewEnumerator3")) (Utilities|Select :Index _tiley :Option%200 "NewEnumerator1" :Option%201 "NewEnumerator1" :Option%202 "NewEnumerator2" :Option%203 "NewEnumerator2" :Option%204 "NewEnumerator2" :Option%205 "NewEnumerator2" :Option%206 "NewEnumerator0" :Option%207 "NewEnumerator0") true _newsmarttile))))
    (:Completed
      (return))))

(fn PackUpBoard
  (bind (_boardrefout _tilex _tiley _index) (Utilities|ForAllTiles self)
    (:LoopBody
      (bind _packedtilestruct (CallFunction|PiecePack _boardrefout _tilex _tiley))
      (Utilities|Array|SetArrayElem (LocalVariables|Gettemp_array1) _index _packedtilestruct))
    (:Completed
      (return (LocalVariables|Gettemp_array1)))))

(fn UnpackBoard
  (params (TileCollection :type Array%20of%20SAMC%20Tile%20Data%20Struct%20Structures))
  (bind (_boardrefout _tilex _tiley _index) (Utilities|ForAllTiles self)
    (:LoopBody
      (Factories|UseTileFactory1 _boardrefout _tilex _tiley)
      (Factories|UsePieceFactory2 _boardrefout (Utilities|Array|Get(acopy) TileCollection _index)))
    (:Completed
      (return))))